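; Number-guessing game Blueprint in which the player counts a guess up to match a random number.
; BeginPlay picks and displays a random integer below 10, while Space increments the displayed guess, capped at 21, until the game is won.
; A match check, run on Tick and after each increment, reveals win and restart text hidden by the construction script.
; After a win, R calls RestartGame on BP_Gamemode.
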(event `self.ReceiveBeginPlay`
  ;[1 1 1] Picks and Displays Random Number
  (bind _output_get (set `self.RandomInt` (`KismetMathLibrary.RandomInteger` 10)))
  (`TextRenderComponent.K2_SetText` (`self.RandomDisplay`) (`KismetTextLibrary.Conv_IntToText` _output_get)))

(event `self.ReceiveTick`
  (params (DeltaSeconds :type "Float (single-precision)"))
  (bind _returnvalue (== (`self.GuessInt`) (`self.RandomInt`)))
  ;[1 1 1] Guessing Mechanic
  (`TextRenderComponent.K2_SetText` (`self.GuessDisplay`) (`KismetTextLibrary.Conv_IntToText` (stale `Key|SpaceBar` _output_get)) :!label _label)
  ;[1 1 1] Displays Appropriate Text if You Win
  (if _returnvalue
    (`SceneComponent.SetHiddenInGame` (`self.RestartText`) false false)
    (if _returnvalue
      (`SceneComponent.SetHiddenInGame` (`self.WinText`) false false)
      (set `self.bHaveWon?` true))))

(event `Key|SpaceBar`
  (params (Key :type "Key Structure"))
  ;[1 1 1] Guessing Mechanic
  (:`Pressed`
    (if (< (`self.GuessInt`) 21)
      (if (not (`self.bHaveWon?`))
        (bind _output_get (set `self.GuessInt` (+ (`self.GuessInt`) 1)))
        (goto _label)))))

(event `Key|R`
  (params (Key :type "Key Structure"))
  (:`Pressed`
    (if (`self.bHaveWon?`)
      (bind _asbp_gamemode (cast `/Game/Blueprints/BP_Gamemode` (`GameplayStatics.GetGameMode`))
        (:`then`
          (`GameMode.RestartGame` _asbp_gamemode))
        (:`CastFailed`
          (`KismetSystemLibrary.PrintString` "Cast failed"))))))

(fn `UserConstructionScript`
  ;[1 1 1] Hides Win and Restart Text At Beginning of Game
  (`SceneComponent.SetHiddenInGame` (`self.WinText`) true false)
  (`SceneComponent.SetHiddenInGame` (`self.RestartText`) true false))